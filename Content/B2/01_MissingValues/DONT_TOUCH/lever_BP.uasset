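; Lever actor that opens and closes a linked door when the third-person character walks into its trigger box.
; While the lever is activable, each overlap alternates through a FlipFlop between on and off.
; Each state sets IsOn, flips the Cube handle's rotation, posts a HUD notification and tells MyDoor to open or close.
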(event `self.Box.OnComponentBeginOverlap`
  (params (OverlappedComponent :type "PrimitiveComponent Object Reference") (OtherActor :type "Actor Object Reference") (OtherComp :type "PrimitiveComponent Object Reference") (OtherBodyIndex :type Integer) (bFromSweep :type Boolean) (SweepResult :type "HitResult Structure (by ref)"))
  (cast `/Game/ThirdPerson/Blueprints/BP_ThirdPersonCharacter` OtherActor)
  (if (`self.isActivable`)
    (`/Engine/EditorBlueprintResources/StandardMacros.FlipFlop`
      (:`A`
        (set `self.isOn` true)
        (message `/Game/DEV/UI/BPI_Interface.notif` (`PlayerController.GetHUD` (`GameplayStatics.GetPlayerController` 0)) "Lever On")
        (`SceneComponent.K2_SetRelativeRotation` (`self.Cube`) (struct :`Yaw` 180.0) false false)
        (`/Game/B2/01_MissingValues/DONT_TOUCH/door_Lvr_BP.OpenDoor` (`self.myDoor`) true))
      (:`B`
        (set `self.isOn` false)
        (message `/Game/DEV/UI/BPI_Interface.notif` (`PlayerController.GetHUD` (`GameplayStatics.GetPlayerController` 0)) "Lever Off")
        (`SceneComponent.K2_SetRelativeRotation` (`self.Cube`) (struct) false false)
        (`/Game/B2/01_MissingValues/DONT_TOUCH/door_Lvr_BP.OpenDoor` (`self.myDoor`) false)))))

(fn `UserConstructionScript`)