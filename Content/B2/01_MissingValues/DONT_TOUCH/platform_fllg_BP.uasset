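; A falling platform actor that drops after the third-person character steps into its trigger box, then returns to its start position.
; BeginPlay caches the Cube's world location.
; On overlap, it waits FallingDelay, enables physics on the Cube, then after a fixed pause disables physics and moves it back.
; The reset restores location only, leaving any rotation picked up during the fall.
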(event `self.ReceiveBeginPlay`
  (set `self.originLoc` (`SceneComponent.K2_GetComponentLocation` (`self.Cube`))))

(event `self.Box.OnComponentBeginOverlap`
  (params (OverlappedComponent :type "PrimitiveComponent Object Reference") (OtherActor :type "Actor Object Reference") (OtherComp :type "PrimitiveComponent Object Reference") (OtherBodyIndex :type Integer) (bFromSweep :type Boolean) (SweepResult :type "HitResult Structure (by ref)"))
  (cast `/Game/ThirdPerson/Blueprints/BP_ThirdPersonCharacter` OtherActor)
  (`KismetSystemLibrary.Delay` (`self.fallingDelay`))
  (`PrimitiveComponent.SetSimulatePhysics` (`self.Cube`) true)
  (`KismetSystemLibrary.Delay` 2.0)
  (`PrimitiveComponent.SetSimulatePhysics` (`self.Cube`) false)
  (`SceneComponent.K2_SetWorldLocation` (`self.Cube`) (`self.originLoc`) false false))

(fn `UserConstructionScript`)