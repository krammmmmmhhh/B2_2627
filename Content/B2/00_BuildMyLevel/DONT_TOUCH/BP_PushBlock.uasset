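; BP_PushBlock is a looping piston-style hazard that launches characters along the actor's up vector.
; After a random start delay, two timelines extend its scene component along relative Z, pause, then retract it and repeat.
; An event track on the push timeline briefly enables the Box trigger, whose overlap applies a PushForce-scaled velocity-change impulse to the character's movement component.
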(event `self.ReceiveBeginPlay`
  (`PrimitiveComponent.SetCollisionEnabled` (`self.Box`) "NoCollision")
  (`KismetSystemLibrary.Delay` (`KismetMathLibrary.RandomFloatInRange` 0.0 2.0))
  (bind (_direction _pushblockalpha) (`Timeline|TL_PushBlock` :!via `PlayFromStart` :!label _label)
    (:`Update`
      (`SceneComponent.K2_SetRelativeLocation` (`self.Scene`) (`KismetMathLibrary.MakeVector` 0.0 0.0 (`KismetMathLibrary.Lerp` 0.0 300.0 _pushblockalpha)) false false))
    (:`Finished`
      (`KismetSystemLibrary.Delay` 2.0)
      (bind (_direction_2 _pushblockalpha_2) (`Timeline|TL_ResetPushBlock` :!via `PlayFromStart`)
        (:`Update`
          (`SceneComponent.K2_SetRelativeLocation` (`self.Scene`) (`KismetMathLibrary.MakeVector` 0.0 0.0 (`KismetMathLibrary.Lerp` 300.0 0.0 _pushblockalpha_2)) false false))
        (:`Finished`
          (goto _label :!via `PlayFromStart`))))
    (:`EnableCollision`
      (`PrimitiveComponent.SetCollisionEnabled` (`self.Box`) "QueryOnly")
      (`KismetSystemLibrary.Delay` 0.1)
      (`PrimitiveComponent.SetCollisionEnabled` (`self.Box`) "NoCollision"))))

(event `self.Box.OnComponentBeginOverlap`
  (params (OverlappedComponent :type "PrimitiveComponent Object Reference") (OtherActor :type "Actor Object Reference") (OtherComp :type "PrimitiveComponent Object Reference") (OtherBodyIndex :type Integer) (bFromSweep :type Boolean) (SweepResult :type "HitResult Structure (by ref)"))
  (bind _ascharacter (cast `Character` OtherActor))
  (`CharacterMovementComponent.AddImpulse` (`Character.CharacterMovement` _ascharacter) (* (`self.GetActorUpVector`) (`self.PushForce`)) true))

(fn `UserConstructionScript`)