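; EndCheckpoint_BP is the level's finish trigger, which checks whether every checkpoint was reached.
; On BeginPlay it caches all Checkpoint_BP actors.
; When a BP_ThirdPersonCharacter enters its Box, it looks for any unreached checkpoint and shows a retry or completion message through the HUD.
; Either result moves the character's CheckpointLoc to this actor, and leaving the Box clears the missing-checkpoint flag.
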(event `self.ReceiveBeginPlay`
  (bind _outactors (`GameplayStatics.GetAllActorsOfClass` "/Game/B2/00_BuildMyLevel/DONT_TOUCH/Checkpoint_BP.Checkpoint_BP_C"))
  (set `self.checkPointActors` _outactors))

(event `self.Box.OnComponentBeginOverlap`
  (params (OverlappedComponent :type "PrimitiveComponent Object Reference") (OtherActor :type "Actor Object Reference") (OtherComp :type "PrimitiveComponent Object Reference") (OtherBodyIndex :type Integer) (bFromSweep :type Boolean) (SweepResult :type "HitResult Structure (by ref)"))
  (bind _asbp_third_person_character (cast `/Game/ThirdPerson/Blueprints/BP_ThirdPersonCharacter` OtherActor))
  (for _array_element (`self.checkPointActors`)
    (if (not (`/Game/B2/00_BuildMyLevel/DONT_TOUCH/Checkpoint_BP.checkpointReached` _array_element))
      (set `self.lackCheckpoint` true)
      (break)))
  (if (`self.lackCheckpoint`)
    (set `/Game/ThirdPerson/Blueprints/BP_ThirdPersonCharacter.checkpointLoc` (`self.K2_GetActorLocation`) _asbp_third_person_character)
    (message `/Game/DEV/UI/BPI_Interface.notif` (`PlayerController.GetHUD` (`GameplayStatics.GetPlayerController` 0)) "You didn't get all checkpoints ! Try again !")
    (else
      (set `/Game/ThirdPerson/Blueprints/BP_ThirdPersonCharacter.checkpointLoc` (`self.K2_GetActorLocation`) _asbp_third_person_character)
      (message `/Game/DEV/UI/BPI_Interface.notif` (`PlayerController.GetHUD` (`GameplayStatics.GetPlayerController` 0)) "Reached the end ! GG"))))

(event `self.Box.OnComponentEndOverlap`
  (params (OverlappedComponent :type "PrimitiveComponent Object Reference") (OtherActor :type "Actor Object Reference") (OtherComp :type "PrimitiveComponent Object Reference") (OtherBodyIndex :type Integer))
  (cast `/Game/ThirdPerson/Blueprints/BP_ThirdPersonCharacter` OtherActor)
  (set `self.lackCheckpoint` false))

(fn `UserConstructionScript`)