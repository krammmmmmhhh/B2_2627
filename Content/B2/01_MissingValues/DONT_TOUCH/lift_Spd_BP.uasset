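; Lift actor that raises its Cube at a configurable Speed and kills the player on contact with its Box trigger.
; On BeginPlay it caches the cube's location, then a timeline with Speed as play rate lerps it along a fixed vertical offset.
; When the third-person character overlaps the Box, it finds the Killzone_BP actor, assigns that character as Player and calls DEAD.
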(event `self.ReceiveBeginPlay`
  (bind _originloc (`self.originLoc`))
  (set `self.originLoc` (`SceneComponent.K2_GetComponentLocation` (`self.Cube`)))
  (`TimelineComponent.SetPlayRate` (`self.TL_MOVE`) (`self.speed`))
  (bind (_direction _time) (`Timeline|TL_MOVE` :!via `PlayFromStart`)
    (:`Update`
      (`SceneComponent.K2_SetWorldLocation` (`self.Cube`) (`KismetMathLibrary.VLerp` _originloc (+ _originloc (0.0 0.0 1000.0)) _time) false false))))

(event `self.Box.OnComponentBeginOverlap`
  (params (OverlappedComponent :type "PrimitiveComponent Object Reference") (OtherActor :type "Actor Object Reference") (OtherComp :type "PrimitiveComponent Object Reference") (OtherBodyIndex :type Integer) (bFromSweep :type Boolean) (SweepResult :type "HitResult Structure (by ref)"))
  (bind _asbp_third_person_character (cast `/Game/ThirdPerson/Blueprints/BP_ThirdPersonCharacter` OtherActor))
  (bind _returnvalue (`GameplayStatics.GetActorOfClass` "/Game/B2/00_BuildMyLevel/DONT_TOUCH/Killzone_BP.Killzone_BP_C"))
  (set `/Game/B2/00_BuildMyLevel/DONT_TOUCH/Killzone_BP.player` _asbp_third_person_character _returnvalue)
  (`/Game/B2/00_BuildMyLevel/DONT_TOUCH/Killzone_BP.DEAD` _returnvalue))

(fn `UserConstructionScript`)