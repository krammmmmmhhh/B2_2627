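; BP_WindZone is a wind volume that pushes the player along the zone's up vector.
; A non-excluded Character entering it starts a looping timer, and one leaving clears it.
; The timer's event presumably runs AddWindForce, a mass-independent velocity impulse scaled by WindForce.
; The impulse always targets the BP_ThirdPersonCharacter cached at BeginPlay, whichever Character overlaps.
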(event `self.ReceiveBeginPlay`
  (bind _returnvalue (`GameplayStatics.GetActorOfClass` "/Game/ThirdPerson/Blueprints/BP_ThirdPersonCharacter.BP_ThirdPersonCharacter_C"))
  (set `self.Player` _returnvalue))

(event `self.ReceiveActorBeginOverlap`
  (params (OtherActor :type "Actor Object Reference"))
  (if (not (`self.ActorHasTag` OtherActor (`self.Exclusion Tag`)))
    (cast `Character` OtherActor)
    (bind _returnvalue (`KismetSystemLibrary.K2_SetTimerDelegate` (`|CreateDelegate` :!event `AddWindForce`) 0.1 true))
    (set `self.WindTimer` _returnvalue)))

(event `self.ReceiveActorEndOverlap`
  (params (OtherActor :type "Actor Object Reference"))
  (if (not (`self.ActorHasTag` OtherActor (`self.Exclusion Tag`)))
    (cast `Character` OtherActor)
    (`KismetSystemLibrary.K2_ClearAndInvalidateTimerHandle` (`self.WindTimer`))))

(event `AddWindForce`
  (`CharacterMovementComponent.AddImpulse` (`Character.CharacterMovement` (`self.Player`)) (* (`self.GetActorUpVector`) (`self.WindForce`)) true))

(fn `UserConstructionScript`)