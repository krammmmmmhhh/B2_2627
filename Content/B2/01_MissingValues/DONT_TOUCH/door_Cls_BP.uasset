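; Door actor that slides shut when the player's third-person character enters its Box trigger.
; The overlap starts the Closing event, whose timeline lerps the Door's relative location downward from raised to lowered, without sweep.
; The same overlap sends a "The Door is closing" notification to the first player's HUD.
; BeginPlay sets the timeline play rate from ClosingSpeed divided by ten; nothing reopens the door.
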(event `self.ReceiveBeginPlay`
  (`TimelineComponent.SetPlayRate` (`self.TL_Closing`) (/ (`self.closingSpeed`) 10.0)))

(event `Closing`
  (bind (_direction _time) (`Timeline|TL_Closing` :!via `PlayFromStart`)
    (:`Update`
      (`SceneComponent.K2_SetRelativeLocation` (`self.door`) (`KismetMathLibrary.VLerp` (0.0 0.0 550.0) (0.0 0.0 150.0) _time) false false))))

(event `self.Box.OnComponentBeginOverlap`
  (params (OverlappedComponent :type "PrimitiveComponent Object Reference") (OtherActor :type "Actor Object Reference") (OtherComp :type "PrimitiveComponent Object Reference") (OtherBodyIndex :type Integer) (bFromSweep :type Boolean) (SweepResult :type "HitResult Structure (by ref)"))
  (cast `/Game/ThirdPerson/Blueprints/BP_ThirdPersonCharacter` OtherActor)
  (`self.Closing`)
  (message `/Game/DEV/UI/BPI_Interface.notif` (`PlayerController.GetHUD` (`GameplayStatics.GetPlayerController` 0)) (`|FormatText` "The Door is closing")))

(fn `UserConstructionScript`)