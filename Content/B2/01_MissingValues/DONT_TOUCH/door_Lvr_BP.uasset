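; Door actor that opens or closes when its OpenDoor event is called with an Open flag.
; Opening is instant and unanimated: the Door component is hidden and its collision disabled, while closing shows it and restores query and physics collision.
; Each call also sends an open or close status message to the first player's HUD through NotifMessage.
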(event `OpenDoor`
  (params (open :type Boolean))
  (bind _door (`self.door`))
  (`SceneComponent.SetVisibility` _door (not open) false)
  (if open
    (`PrimitiveComponent.SetCollisionEnabled` _door "NoCollision")
    (else
      (`PrimitiveComponent.SetCollisionEnabled` _door "QueryAndPhysics")))
  (message `/Game/DEV/UI/BPI_Interface.notif` (`PlayerController.GetHUD` (`GameplayStatics.GetPlayerController` 0)) (`|FormatText` "Door is {0}" (`KismetMathLibrary.SelectText` "Open" "Close" open))))

(fn `UserConstructionScript`)