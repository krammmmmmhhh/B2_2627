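; Platform actor that repeatedly appears and disappears during play.
; A Switch event shows the Cube with collision, waits EnableFor, hides it without collision, waits DisableFor, then calls itself to loop.
; BeginPlay starts the loop after a random delay of up to three seconds, so separate instances fall out of sync.
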(event `self.ReceiveBeginPlay`
  (`KismetSystemLibrary.Delay` (`KismetMathLibrary.RandomFloatInRange` 0.0 3.0))
  (`self.Switch`))

(event `Switch`
  (`PrimitiveComponent.SetCollisionEnabled` (`self.Cube`) "QueryAndPhysics")
  (`SceneComponent.SetVisibility` (`self.Cube`) true false)
  (`KismetSystemLibrary.Delay` (`self.enableFor`))
  (`PrimitiveComponent.SetCollisionEnabled` (`self.Cube`) "NoCollision")
  (`SceneComponent.SetVisibility` (`self.Cube`) false false)
  (`KismetSystemLibrary.Delay` (`self.disableFor`))
  (`self.Switch`))

(event `self.ReceiveTick`
  (params (DeltaSeconds :type "Float (single-precision)")))

(fn `UserConstructionScript`)