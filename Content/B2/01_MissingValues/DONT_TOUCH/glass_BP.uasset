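; Glass actor that the player can destroy by interacting with it from inside its Box trigger.
; On BeginPlay it caches the player controller, passes it its InputToInteract value and switches Tick off.
; Box overlaps with the third-person character toggle Tick, which polls the controller's InteractKeyPressed flag.
; When the flag is set, the glass sends a "Glass Destroyed" HUD notification and destroys itself.
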(event `self.ReceiveBeginPlay`
  (bind _asbp_third_person_player_controller (cast `/Game/ThirdPerson/Blueprints/BP_ThirdPersonPlayerController` (`GameplayStatics.GetPlayerController` 0)))
  (bind _output_get (set `self.controller` _asbp_third_person_player_controller))
  (set `/Game/ThirdPerson/Blueprints/BP_ThirdPersonPlayerController.inputToInteract` (`self.inputToInteract`) _output_get)
  (`self.SetActorTickEnabled` false))

(event `self.ReceiveTick`
  (params (DeltaSeconds :type "Float (single-precision)"))
  (if (`/Game/ThirdPerson/Blueprints/BP_ThirdPersonPlayerController.interactKeyPressed` (`self.controller`))
    (message `/Game/DEV/UI/BPI_Interface.notif` (`PlayerController.GetHUD` (`GameplayStatics.GetPlayerController` 0)) (`|FormatText` "Glass Destroyed"))
    (`self.K2_DestroyActor`)))

(event `self.Box.OnComponentBeginOverlap`
  (params (OverlappedComponent :type "PrimitiveComponent Object Reference") (OtherActor :type "Actor Object Reference") (OtherComp :type "PrimitiveComponent Object Reference") (OtherBodyIndex :type Integer) (bFromSweep :type Boolean) (SweepResult :type "HitResult Structure (by ref)"))
  (cast `/Game/ThirdPerson/Blueprints/BP_ThirdPersonCharacter` OtherActor)
  (`self.SetActorTickEnabled` true))

(event `self.Box.OnComponentEndOverlap`
  (params (OverlappedComponent :type "PrimitiveComponent Object Reference") (OtherActor :type "Actor Object Reference") (OtherComp :type "PrimitiveComponent Object Reference") (OtherBodyIndex :type Integer))
  (cast `/Game/ThirdPerson/Blueprints/BP_ThirdPersonCharacter` OtherActor)
  (`self.SetActorTickEnabled` false))

(fn `UserConstructionScript`)