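; Speed booster actor that temporarily raises the walk speed of a character overlapping it.
; BeginPlay caches the first BP_ThirdPersonCharacter and its initial MaxWalkSpeed.
; Overlap sets MaxSpeed on any Character lacking the exclusion tag and starts a three-second timer.
; MaxSpeedReset restores the initial speed only on the cached player, not the overlapping character, and clears the timer.
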(event `self.ReceiveBeginPlay`
  (bind _returnvalue (`GameplayStatics.GetActorOfClass` "/Game/ThirdPerson/Blueprints/BP_ThirdPersonCharacter.BP_ThirdPersonCharacter_C"))
  (bind _output_get (set `self.Player` _returnvalue))
  (set `self.InitSpeed` (`CharacterMovementComponent.MaxWalkSpeed` (`Character.CharacterMovement` _output_get))))

(event `self.ReceiveActorBeginOverlap`
  (params (OtherActor :type "Actor Object Reference"))
  (if (not (`self.ActorHasTag` OtherActor (`self.Exclusion Tag`)))
    (bind _ascharacter (cast `Character` OtherActor))
    (set `CharacterMovementComponent.MaxWalkSpeed` (`self.Max Speed`) (`Character.CharacterMovement` _ascharacter))
    (bind _returnvalue (`KismetSystemLibrary.K2_SetTimerDelegate` (`|CreateDelegate` :!event `MaxSpeedReset`) 3.0))
    (set `self.SpeedTimer` _returnvalue)))

(event `MaxSpeedReset`
  (set `CharacterMovementComponent.MaxWalkSpeed` (`self.InitSpeed`) (`Character.CharacterMovement` (`self.Player`)))
  (`KismetSystemLibrary.K2_ClearAndInvalidateTimerHandle` (`self.SpeedTimer`)))

(fn `UserConstructionScript`)